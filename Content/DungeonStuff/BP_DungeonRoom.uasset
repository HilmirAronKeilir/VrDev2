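; BP_DungeonRoom is a dungeon room actor that builds its floor grid at runtime.
; On BeginPlay it picks a random row from Data_DungeonType and uses its X and Y as grid dimensions, adding evenly spaced BP_DungeonTile components.
; After a short delay it checks for overlapping BP_DungeonRoom actors and prints a debug "Island" message when it finds none.
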(event EventBeginPlay
  (bind _outrownames (DataTable|GetDataTableRowNames "/Game/DataStuff/Data_DungeonType.Data_DungeonType"))
  (bind _returnvalue (Utilities|GetDataTableRow "/Game/DataStuff/Data_DungeonType.Data_DungeonType" (.OutItem (Utilities|Array|Random _outrownames)))
    (:then
      (for _index (range 0 (- (.x _returnvalue) 1))
        (for _index_2 (range 0 (- (.y _returnvalue) 1))
          (Game|AddComponentbyClass "/Game/DungeonStuff/BP_DungeonTile.BP_DungeonTile_C" false (Math|Transform|MakeTransform (Math|Vector|MakeVector (* _index 1e+02) (* _index_2 1e+02) 0.0) "0, 0, 0" "1.000000,1.000000,1.000000"))))
      (Utilities|FlowControl|Delay 1.5)
      (if (== (Utilities|Array|Length (Collision|GetOverlappingActors "BP_DungeonRoom_C" :!class /Script/Engine.Actor)) 0)
        (Development|PrintString "Island")))))

(fn ConstructionScript)